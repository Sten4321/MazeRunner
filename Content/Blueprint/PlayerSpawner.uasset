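; PlayerSpawner is an actor that spawns the player once dungeon generation has finished.
; Until PlayerSpawned is set, Tick looks up the first DungeonGenerator in the level and polls its Done flag.
; A DoOnce then waits briefly, spawns Player_BP at a random point inside the PlayerSpawn box, adjusting for collisions but always spawning, and sets the flag to end polling.
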(event `self.ReceiveTick`
  (params (DeltaSeconds :type "Float (single-precision)"))
  (bind _playerspawn (`self.PlayerSpawn`))
  (if (not (`self.PlayerSpawned`))
    (bind _outactors (`GameplayStatics.GetAllActorsOfClass` "/Game/DungeonGenerator/Blueprints/DungeonGenerator.DungeonGenerator_C"))
    (bind _output (`|GetArrayItem` _outactors))
    (`/Engine/EditorBlueprintResources/StandardMacros.IsValid` _output
      (:`Is Valid`
        (if (`/Game/DungeonGenerator/Blueprints/DungeonGenerator.Done` _output)
          (`/Engine/EditorBlueprintResources/StandardMacros.DoOnce` false
            (:`Completed`
              (`KismetSystemLibrary.Delay` 0.5)
              (`|SpawnActorFromClass` "/Game/FirstPersonCPP/Blueprints/Player_BP.Player_BP_C" (`KismetMathLibrary.Conv_VectorToTransform` (`KismetMathLibrary.RandomPointInBoundingBox` (`SceneComponent.K2_GetComponentLocation` _playerspawn) (`BoxComponent.GetScaledBoxExtent` _playerspawn))) "AdjustIfPossibleButAlwaysSpawn" "OverrideRootScale" null null)
              (set `self.PlayerSpawned` true))))))))

(fn `UserConstructionScript`)