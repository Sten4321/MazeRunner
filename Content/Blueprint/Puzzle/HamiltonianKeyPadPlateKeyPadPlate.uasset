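; Pressure plate for a Hamiltonian keypad puzzle, toggled when the player steps onto its overlap box.
; Entering an inactive plate activates it, while re-entering an active one deactivates it and loops over PuzzlePlates to clear activation, resetting progress.
; Tick polls IsActivated every frame to show gold metal when active and copper when inactive.
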(event `self.ReceiveTick`
  (params (DeltaSeconds :type "Float (single-precision)"))
  (bind _plate (`self.Plate`))
  (if (`self.IsActivated`)
    (`PrimitiveComponent.SetMaterial` _plate 0 "/Game/StarterContent/Materials/M_Metal_Gold.M_Metal_Gold")
    (else
      (`PrimitiveComponent.SetMaterial` _plate 0 "/Game/StarterContent/Materials/M_Metal_Copper.M_Metal_Copper"))))

(event `self.Box.OnComponentBeginOverlap`
  (params (OverlappedComponent :type "PrimitiveComponent Object Reference") (OtherActor :type "Actor Object Reference") (OtherComp :type "PrimitiveComponent Object Reference") (OtherBodyIndex :type Integer) (bFromSweep :type Boolean) (SweepResult :type "HitResult Structure (by ref)"))
  (if (== (`GameplayStatics.GetObjectClass` OtherActor) "/Game/FirstPersonCPP/Blueprints/Player_BP.Player_BP_C")
    (if (`self.IsActivated`)
      (set `self.IsActivated` false)
      (for _ (`self.PuzzlePlates`)
        (set `self.IsActivated` false))
      (else
        (set `self.IsActivated` true)))))

(fn `UserConstructionScript`)