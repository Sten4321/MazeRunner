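; Floor plate for a Hamiltonian-style puzzle that opens a door when all linked plates are active.
; Player overlap toggles the plate, and Tick swaps its material between gold and copper to show state.
; Activation checks PuzzlePlates and updates Door1; deactivation closes it, while solving sets OpenDoor on linked plates to lock the puzzle.
; The construction script's auto-lookup of plates and door is disconnected and never runs.
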(event `self.ReceiveTick`
  (params (DeltaSeconds :type "Float (single-precision)"))
  (bind _plate (`self.Plate`))
  (if (`self.IsActivated`)
    (`PrimitiveComponent.SetMaterial` _plate 0 "/Game/StarterContent/Materials/M_Metal_Gold.M_Metal_Gold")
    (else
      (`PrimitiveComponent.SetMaterial` _plate 0 "/Game/StarterContent/Materials/M_Metal_Copper.M_Metal_Copper"))))

(event `self.Box.OnComponentBeginOverlap`
  (params (OverlappedComponent :type "PrimitiveComponent Object Reference") (OtherActor :type "Actor Object Reference") (OtherComp :type "PrimitiveComponent Object Reference") (OtherBodyIndex :type Integer) (bFromSweep :type Boolean) (SweepResult :type "HitResult Structure (by ref)"))
  (if (== (`GameplayStatics.GetObjectClass` OtherActor) "/Game/FirstPersonCPP/Blueprints/Player_BP.Player_BP_C")
    (if (`self.OpenDoor`)
      _
      (elif (`self.IsActivated`)
        (set `self.IsActivated` false)
        ;[1 1 1] CloseDoor
        (for _ (`self.PuzzlePlates`)
          (set `self.IsActivated` false)
          (set `/Game/Blueprint/Door_Blueprint.Open` false (`self.Door1`)))
        (else
          (set `self.IsActivated` true)
          (set `self.OpenDoor` true)
          ;[1 1 1] See if all is activated
          (for _array_element (`self.PuzzlePlates`)
            (if (not (`/Game/Blueprint/Puzzle/HamiltonianKeyPadPlate.IsActivated` _array_element))
              (set `self.OpenDoor` false)
              (break)))
          (`/Game/Blueprint/Door_Blueprint.SetOpen` (`self.Door1`) (`self.OpenDoor`))
          ;[1 1 1] Disable Puzzle
          (if (`self.OpenDoor`)
            (for _array_element_2 (`self.PuzzlePlates`)
              (set `/Game/Blueprint/Puzzle/HamiltonianKeyPadPlate.OpenDoor` true _array_element_2))))))))

(fn `UserConstructionScript`)