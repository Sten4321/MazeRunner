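; Pitfall trap Actor that opens a spike pit beneath the player.
; When the player pawn overlaps the trigger, a one-second delay runs, then the trigger, pressure plate and disappearing floor components are destroyed to reveal the pit.
; Hits on the spike floor apply heavy damage to any damageable actor, with the trap as damage causer.
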(event `self.TrapTrigger.OnComponentBeginOverlap`
  (params (OverlappedComponent :type "PrimitiveComponent Object Reference") (OtherActor :type "Actor Object Reference") (OtherComp :type "PrimitiveComponent Object Reference") (OtherBodyIndex :type Integer) (bFromSweep :type Boolean) (SweepResult :type "HitResult Structure (by ref)"))
  ;[1 1 1] Check If player
  (if (== OtherActor (`GameplayStatics.GetPlayerPawn` 0))
    (`KismetSystemLibrary.Delay` 1.0)
    ;[1 1 1] Reveal PitTrap
    (`ActorComponent.K2_DestroyComponent` (`self.TrapTrigger`))
    (`ActorComponent.K2_DestroyComponent` (`self.PressurePlate`))
    (`ActorComponent.K2_DestroyComponent` (`self.DissapiringFloor`))))

(event `self.SpikeFloor.OnComponentHit`
  (params (HitComponent :type "PrimitiveComponent Object Reference") (OtherActor :type "Actor Object Reference") (OtherComp :type "PrimitiveComponent Object Reference") (NormalImpulse :type "Vector Structure") (Hit :type "HitResult Structure (by ref)"))
  ;[1 1 1] Spike Deals Damage
  (if (`Actor.bCanBeDamaged` OtherActor)
    (`GameplayStatics.ApplyDamage` OtherActor 500.0 null (`ActorComponent.GetOwner` (`self.SpikeFloor`)))))

(fn `UserConstructionScript`)