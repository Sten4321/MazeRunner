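; Spike trap actor that shoots spikes up when a damageable actor enters its trigger, then retracts them.
; The trigger disables its collision, waits briefly, and a timeline lerps the spikes between their start position and a raised one.
; A Done flag reverses the timeline once, then re-enables the trigger when the spikes are back down.
; Each spike mesh applies fixed damage to damageable actors it hits.
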(event `self.ReceiveBeginPlay`
  (bind _output_get (set `self.StartPos` (`SceneComponent.K2_GetComponentLocation` (`self.Spikes`))))
  (set `self.EndPos` (+ _output_get (0.0 0.0 200.0))))

(event `self.TrapTrigger.OnComponentBeginOverlap`
  (params (OverlappedComponent :type "PrimitiveComponent Object Reference") (OtherActor :type "Actor Object Reference") (OtherComp :type "PrimitiveComponent Object Reference") (OtherBodyIndex :type Integer) (bFromSweep :type Boolean) (SweepResult :type "HitResult Structure (by ref)"))
  ;[1 1 1] Check If pawn can take damage
  (if (`Actor.bCanBeDamaged` OtherActor)
    (`PrimitiveComponent.SetCollisionEnabled` (`self.TrapTrigger`) "NoCollision")
    (`KismetSystemLibrary.Delay` 0.1)
    ;[1 1 1] MoveSpike Up And Down
    (bind (_direction _spiketrapline) (`Timeline|SpikeTrap` :!via `PlayFromStart` :!label _label)
      (:`Update`
        (`SceneComponent.K2_SetWorldLocation` (`self.Spikes`) (`KismetMathLibrary.VLerp` (`self.StartPos`) (`self.EndPos`) _spiketrapline) false false))
      (:`Finished`
        (if (`self.Done`)
          (set `self.Done` false)
          (`PrimitiveComponent.SetCollisionEnabled` (`self.TrapTrigger`) "QueryAndPhysics")
          (else
            (set `self.Done` true)
            (`self.Revert`)))))))

(event `Revert`
  ;[1 1 1] MoveSpike Up And Down
  (if (`self.Done`)
    (goto _label :!via `ReverseFromEnd`)))

(event `self.Spikes.OnComponentHit`
  (params (HitComponent :type "PrimitiveComponent Object Reference") (OtherActor :type "Actor Object Reference") (OtherComp :type "PrimitiveComponent Object Reference") (NormalImpulse :type "Vector Structure") (Hit :type "HitResult Structure (by ref)"))
  ;[1 1 1] Spike Deals Damage
  (if (`Actor.bCanBeDamaged` OtherActor)
    (`GameplayStatics.ApplyDamage` OtherActor 10.0 null (`ActorComponent.GetOwner` (`self.Spikes`)))))

(event `self.Spike1.OnComponentHit`
  (params (HitComponent :type "PrimitiveComponent Object Reference") (OtherActor :type "Actor Object Reference") (OtherComp :type "PrimitiveComponent Object Reference") (NormalImpulse :type "Vector Structure") (Hit :type "HitResult Structure (by ref)"))
  ;[1 1 1] Spike Deals Damage
  (if (`Actor.bCanBeDamaged` OtherActor)
    (`GameplayStatics.ApplyDamage` OtherActor 10.0 null (`ActorComponent.GetOwner` (`self.Spike1`)))))

(event `self.Spike2.OnComponentHit`
  (params (HitComponent :type "PrimitiveComponent Object Reference") (OtherActor :type "Actor Object Reference") (OtherComp :type "PrimitiveComponent Object Reference") (NormalImpulse :type "Vector Structure") (Hit :type "HitResult Structure (by ref)"))
  ;[1 1 1] Spike Deals Damage
  (if (`Actor.bCanBeDamaged` OtherActor)
    (`GameplayStatics.ApplyDamage` OtherActor 10.0 null (`ActorComponent.GetOwner` (`self.Spike2`)))))

(event `self.Spike3.OnComponentHit`
  (params (HitComponent :type "PrimitiveComponent Object Reference") (OtherActor :type "Actor Object Reference") (OtherComp :type "PrimitiveComponent Object Reference") (NormalImpulse :type "Vector Structure") (Hit :type "HitResult Structure (by ref)"))
  ;[1 1 1] Spike Deals Damage
  (if (`Actor.bCanBeDamaged` OtherActor)
    (`GameplayStatics.ApplyDamage` OtherActor 10.0 null (`ActorComponent.GetOwner` (`self.Spike3`)))))

(event `self.Spike4.OnComponentHit`
  (params (HitComponent :type "PrimitiveComponent Object Reference") (OtherActor :type "Actor Object Reference") (OtherComp :type "PrimitiveComponent Object Reference") (NormalImpulse :type "Vector Structure") (Hit :type "HitResult Structure (by ref)"))
  ;[1 1 1] Spike Deals Damage
  (if (`Actor.bCanBeDamaged` OtherActor)
    (`GameplayStatics.ApplyDamage` OtherActor 10.0 null (`ActorComponent.GetOwner` (`self.Spike4`)))))

(fn `UserConstructionScript`)