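; JunkSpawner is a one-shot spawner actor that places a single random junk item within an area.
; On its first tick it calls SpawnJunk, then destroys itself.
; SpawnJunk picks a random class from ArrayOfJunk and spawns it at a random point inside the AreaToSpawn box extent, adjusting for collisions but always spawning.
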(event `self.ReceiveTick`
  (params (DeltaSeconds :type "Float (single-precision)"))
  (`/Engine/EditorBlueprintResources/StandardMacros.DoOnce` false
    (:`Completed`
      (`self.SpawnJunk`)
      (`self.K2_DestroyActor` self))))

(fn `SpawnJunk`
  (bind _arrayofjunk (`self.ArrayOfJunk`))
  (bind _areatospawn (`self.AreaToSpawn`))
  (`|SpawnActorFromClass` (`|GetArrayItem` _arrayofjunk (`KismetMathLibrary.RandomIntegerInRange` 0 (- (`KismetArrayLibrary.Array_Length` _arrayofjunk) 1))) (`KismetMathLibrary.Conv_VectorToTransform` (`KismetMathLibrary.RandomPointInBoundingBox` (`SceneComponent.K2_GetComponentLocation` _areatospawn) (`BoxComponent.GetScaledBoxExtent` _areatospawn))) "AdjustIfPossibleButAlwaysSpawn" "OverrideRootScale" null null))

(fn `UserConstructionScript`)