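; EnemySpawner is an actor that spawns Enemy_BP AI pawns at random points inside its SpawnArea box while the player is nearby.
; Tick waits until the DungeonGenerator reports Done, caching that in WorldGenFinished.
; When the player is within MaxSpawnDistance, it waits SpawnDelay, rechecks the distance and calls SpawnEnemy.
; SpawnEnemy spawns only while the level-wide Enemy_BP count is below MaxEnemies.
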(event `self.ReceiveTick`
  (params (DeltaSeconds :type "Float (single-precision)"))
  (bind _returnvalue (`GameplayStatics.GetPlayerPawn` 0))
  (bind _returnvalue_2 (<= (`KismetMathLibrary.VSize` (- (`self.K2_GetActorLocation` self) (`self.K2_GetActorLocation` _returnvalue))) (`self.MaxSpawnDistance`)))
  (`/Engine/EditorBlueprintResources/StandardMacros.IsValid` _returnvalue
    (:`Is Valid`
      (if (`self.WorldGen Finished`)
        (if _returnvalue_2 :!label _label
          (`KismetSystemLibrary.Delay` (`self.SpawnDelay`))
          (if _returnvalue_2
            (`self.SpawnEnemy`)))
        (else
          (bind _outactors (`GameplayStatics.GetAllActorsOfClass` "/Game/DungeonGenerator/Blueprints/DungeonGenerator.DungeonGenerator_C"))
          (bind _output (`|GetArrayItem` _outactors))
          (`/Engine/EditorBlueprintResources/StandardMacros.IsValid` _output
            (:`Is Valid`
              (if (`/Game/DungeonGenerator/Blueprints/DungeonGenerator.Done` _output)
                (set `self.WorldGen Finished` true)
                (goto _label)))))))))

(fn `SpawnEnemy`
  (bind _spawnarea (`self.SpawnArea`))
  (bind _outactors (`GameplayStatics.GetAllActorsOfClass` "/Game/FirstPersonCPP/Blueprints/Enemy_BP.Enemy_BP_C"))
  (if (< (`KismetArrayLibrary.Array_Length` _outactors) (`self.MaxEnemies`))
    (`AIBlueprintHelperLibrary.SpawnAIFromClass` "/Game/FirstPersonCPP/Blueprints/Enemy_BP.Enemy_BP_C" null (`KismetMathLibrary.RandomPointInBoundingBox` (`SceneComponent.K2_GetComponentLocation` _spawnarea) (`BoxComponent.GetScaledBoxExtent` _spawnarea)))))

(fn `UserConstructionScript`)