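; Enemy AI controller that runs the Guard behavior tree and feeds it sensed targets through a blackboard.
; On BeginPlay it initializes the EnemyData blackboard, starts the tree and caches the blackboard component.
; AI perception updates write any successfully sensed actor to EnemyKey and clear the key when sensing fails.
; A Player tag check exists but is unused, so targets are not filtered by tag.
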(event `self.ReceiveBeginPlay`
  (bind _blackboardcomponent (`self.UseBlackboard` "/Game/BehaviorTree/EnemyData.EnemyData"))
  (`self.RunBehaviorTree` "/Game/BehaviorTree/Guard.Guard")
  (set `self.Blackboard_Comp` _blackboardcomponent))

(event `self.AIPerception.OnTargetPerceptionUpdated`
  (params (Actor :type "Actor Object Reference") (Stimulus :type "AIStimulus Structure"))
  (bind _enemykey (`self.EnemyKey`))
  (bind _blackboard_comp (`self.Blackboard_Comp`))
  ;[1 1 1] React with senses
  (if (`.bSuccessfullySensed` (break `AIStimulus` Stimulus))
    (`BlackboardComponent.SetValueAsObject` _blackboard_comp _enemykey Actor)
    (else
      (`BlackboardComponent.ClearValue` _blackboard_comp _enemykey))))

(fn `UserConstructionScript`)