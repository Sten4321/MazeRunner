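; Dungeon generator layout Blueprint that checks whether the key EndTile was spawned in the generated layout.
; On ModifyLayout it scans all DungeonTile actors, compares each tile's map path to the hardcoded EndTile map and stops at the first match.
; It prints a confirmation when found, otherwise only the current level name.
; The intended retry is unfinished: the generator restart (noted as not working) and level reload are disconnected.
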(event `self.ModifyLayout`
  ;[1 1 1] Get all placed tiles
  (bind _outactors (`GameplayStatics.GetAllActorsOfClass` "/Game/DungeonGenerator/Blueprints/DungeonTile.DungeonTile_C"))
  (for _array_element _outactors :!label _label
    (if (`KismetStringLibrary.EqualEqual_StrStr` (`.Map_2_6871C05D4C41DBC201A03D8195C1B201` (break `/Game/DungeonGenerator/Data/TileData` (`/Game/DungeonGenerator/Blueprints/DungeonTile.TileData` _array_element))) "/Game/Maps/TileMaps/EndTile/EndTile")
      (set `self.FoundEndTile` true)
      (`self.Done`)))
  ;[1 1 1] Restart Generater if the keyTiles are not spawned
  (if (`self.FoundEndTile`)
    (`KismetSystemLibrary.PrintString` "EndTile Spawned" true true (struct :`G` 0.66 :`B` 1.0 :`A` 1.0) 5.0)
    (else
      (bind _returnvalue (`GameplayStatics.GetCurrentLevelName` true))
      (`KismetSystemLibrary.PrintString` _returnvalue true true (struct :`G` 0.66 :`B` 1.0 :`A` 1.0) 5.0))))

(event `Done`
  (goto _label :!via `Break`))

(fn `UserConstructionScript`
  (`parent.UserConstructionScript`))